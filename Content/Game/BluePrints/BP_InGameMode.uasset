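; In-game game mode Blueprint that manages the HUD and the end screen shown when a car hit occurs.
; On BeginPlay it binds the car-hit event, displays the UI widget, and creates a menu widget without displaying it.
; A hit swaps the HUD for the end widget, where a timeline animates the score by feeding its output and GameTime through a Lerp from zero.
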(event `self.ReceiveBeginPlay`
  (add `self.HitCarEvent` (delegate `OnCarHitEvent`))
  ;[0 0.02152 0.1719] UIの表示
  (bind _returnvalue (`|CreateWidget` "/Game/Game/Widget/WBP_UI.WBP_UI_C"))
  (bind _output_get (set `self.WBP_UI` _returnvalue))
  (`UserWidget.AddToViewport` _output_get 0)
  (bind _returnvalue_2 (`|CreateWidget` "/Game/Game/Widget/WBP_GsmeMenu.WBP_GsmeMenu_C"))
  (set `self.WBP_Menu` _returnvalue_2))

(event `OnCarHitEvent`
  ;[0.009562 0.1562 0] 車がヒットした後の処理
  (`Widget.RemoveFromParent` (`self.WBP_UI`))
  (bind _returnvalue (`|CreateWidget` "/Game/Game/Widget/WBP_End.WBP_End_C"))
  (`UserWidget.AddToViewport` _returnvalue 0)
  (bind (_direction _time) (`Timeline|Score用`)
    (:`Update`
      (`/Game/Game/Widget/WBP_End.UpdateScore` _returnvalue (`KismetMathLibrary.Lerp` 0.0 _time (`self.GameTime`))))))

(fn `UserConstructionScript`)